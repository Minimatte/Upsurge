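; Ship class-system component (WIP) that spawns and attaches weapons to its owning BP_Ship on BeginPlay.
; SpawnWeapons loops over every ShipMesh socket, choosing PrimaryWeapon when the name's split left part equals "Primary", otherwise SecondaryWeapon.
; Each weapon spawns at its socket, owned and instigated by the ship, joins a primary or secondary reference array, and attaches to the ship.
; The split delimiter is empty.
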(event `self.ReceiveBeginPlay`
  (`self.SpawnTheWeapons`))

(event `SpawnTheWeapons`
  (`self.SpawnWeapons`))

(fn `SpawnWeapons`
  (bind _returnvalue (`self.GetOwner`))
  (bind _aspawn (cast `Pawn` _returnvalue :!pure true))
  (bind _shipmesh (`/Game/BP_Ship.ShipMesh` (cast `/Game/BP_Ship` (`self.GetOwner`) :!pure true)))
  (for _array_element (`SceneComponent.GetAllSocketNames` _shipmesh)
    (if (`KismetStringLibrary.EqualEqual_StrStr` (`KismetStringLibrary.Split` (`KismetStringLibrary.Conv_NameToString` _array_element) " ") "Primary")
      (bind _returnvalue_2 (`SceneComponent.GetSocketTransform` _shipmesh _array_element "RTS_World"))
      (bind _returnvalue_3 (`|SpawnActorFromClass` (`self.PrimaryWeapon`) _returnvalue_2 "AlwaysSpawn" "OverrideRootScale" _returnvalue _aspawn))
      (`KismetArrayLibrary.Array_Add` (`self.PrimaryWeaponsRef`) _returnvalue_3)
      (`self.K2_AttachRootComponentToActor` _returnvalue_3 _returnvalue _array_element "KeepWorldPosition" true)
      (else
        (bind _returnvalue_4 (`|SpawnActorFromClass` (`self.SecondaryWeapon`) _returnvalue_2 "AlwaysSpawn" "OverrideRootScale" _returnvalue _aspawn))
        (`KismetArrayLibrary.Array_Add` (`self.SecondaryWeaponsRef`) _returnvalue_4)
        (`self.K2_AttachRootComponentToActor` _returnvalue_4 _returnvalue _array_element "KeepWorldPosition" true)))))

(fn `UserConstructionScript`)