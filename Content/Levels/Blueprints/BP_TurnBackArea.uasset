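; BP_TurnBackArea is a level volume that marks the battlefield bounds for BP_Ship actors.
; When a valid ship stops overlapping its Box, it flags the ship as OutsideBattlefield and calls DieIn10Seconds on it.
; When a ship begins overlapping again, it only clears that flag, leaving any handling of the pending death to BP_Ship.
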(event `self.Box.OnComponentEndOverlap`
  (params (OtherActor :type "Actor Object Reference") (OtherComp :type "PrimitiveComponent Object Reference") (OtherBodyIndex :type Integer))
  (if (== (`GameplayStatics.GetObjectClass` OtherActor) "/Game/BP_Ship.BP_Ship_C")
    ;[1 1 1] If player is dead or not
    (`/Engine/EditorBlueprintResources/StandardMacros.IsValid` OtherActor
      (:`Is Valid`
        (bind _asbp_ship (cast `/Game/BP_Ship` OtherActor))
        (set `/Game/BP_Ship.outsideBattlefield` true _asbp_ship)
        (`/Game/BP_Ship.DieIn10Seconds` _asbp_ship 10.0)))))

(event `self.Box.OnComponentBeginOverlap`
  (params (OtherActor :type "Actor Object Reference") (OtherComp :type "PrimitiveComponent Object Reference") (OtherBodyIndex :type Integer) (bFromSweep :type Boolean) (SweepResult :type "HitResult Structure (by ref)"))
  (if (== (`GameplayStatics.GetObjectClass` OtherActor) "/Game/BP_Ship.BP_Ship_C")
    (`/Engine/EditorBlueprintResources/StandardMacros.IsValid` OtherActor
      (:`Is Valid`
        (bind _asbp_ship (cast `/Game/BP_Ship` OtherActor))
        (set `/Game/BP_Ship.outsideBattlefield` false _asbp_ship)))))

(fn `UserConstructionScript`)