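; BP_Fan_Networked is a spinning fan hazard that deals lethal damage to any BP_Ship hitting its blade.
; Each tick, the authority rotates the blade by FanSpeed with sweep and stores its world rotation in FanRotation.
; Remote instances apply FanRotation to the blade instead of simulating the spin.
; An attenuated fan sound spawns at the actor's location on BeginPlay.
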(event `self.ReceiveBeginPlay`
  (`GameplayStatics.SpawnSoundAtLocation` "/Game/Sounds/Fans/Fan_Cue.Fan_Cue" (`self.K2_GetActorLocation`) (struct) 2.0 1.0 0.0 "/Game/Sounds/GameSoundAttenuation.GameSoundAttenuation"))

(event `/Game/Levels/Blueprints/BP_Fan.ReceiveTick`
  (params (DeltaSeconds :type "Float (single-precision)"))
  (bind _sm_fan_blade (`self.SM_fan_blade`))
  (`/Engine/EditorBlueprintResources/ActorMacros.Switch Has Authority`
    (:`Authority`
      (`SceneComponent.K2_AddLocalRotation` _sm_fan_blade (`KismetMathLibrary.MakeRotator` 0.0 0.0 (* (`self.FanSpeed`) DeltaSeconds)) true true)
      (set `self.FanRotation` (`SceneComponent.K2_GetComponentRotation` _sm_fan_blade)))
    (:`Remote`
      (`SceneComponent.K2_SetWorldRotation` (`self.SM_fan_blade`) (`self.FanRotation`) false false))))

(event `self.SM_fan_blade.OnComponentHit`
  (params (OtherActor :type "Actor Object Reference") (OtherComp :type "PrimitiveComponent Object Reference") (NormalImpulse :type "Vector Structure") (Hit :type "HitResult Structure (by ref)"))
  (if (== (`GameplayStatics.GetObjectClass` OtherActor) "/Game/BP_Ship.BP_Ship_C")
    (`GameplayStatics.ApplyDamage` OtherActor 9999.0)))

(fn `UserConstructionScript`)