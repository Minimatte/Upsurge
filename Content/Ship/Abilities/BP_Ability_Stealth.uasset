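; Stealth ability for BP_Ship that triggers a material change on the owning ship's mesh.
; OverrideThis casts the owner to BP_Ship and passes it with its ShipMesh through SetVar to the ship's SetMeshMaterial.
; BeginPlay caches and debug-prints the ship when the owner is player 0's character.
; An author note indicates the change is meant to go through a multicast event on the ship.
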(event `self.ReceiveBeginPlay`
  (if (== (`self.GetOwner`) (`GameplayStatics.GetPlayerCharacter` 0))
    (bind _output_get (set `self.ShipMesh` (cast `/Game/BP_Ship` (`self.GetOwner`) :!pure true)))
    (`KismetSystemLibrary.PrintString` (`KismetSystemLibrary.GetDisplayName` _output_get) true true (struct :`R` 1.0 :`G` 0.023671 :`A` 1.0) 123123.0)))

(event `self.OverrideThis`
  (bind _asbp_ship (cast `/Game/BP_Ship` (`self.GetOwner`) :!pure true))
  (`self.SetVar` _asbp_ship (`/Game/BP_Ship.ShipMesh` _asbp_ship)))

(event `SetVar`
  (params (NewParam :type "/Game/BP_Ship Object Reference") (Target :type "PrimitiveComponent Object Reference"))
  ;[1 1 1] Make a custom event in the ship with multicast that this gets
  (`/Game/BP_Ship.setMeshMaterial` NewParam Target))

(fn `UserConstructionScript`
  (`parent.UserConstructionScript`))