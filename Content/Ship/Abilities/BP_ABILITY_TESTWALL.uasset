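; BP_ABILITY_TESTWALL is a ship ability, apparently a test, that spawns a wall ahead of the ability actor.
; The OverrideThis event computes a point 1000 units along the actor's forward vector and passes it, with the actor's rotation, to the spawnWall event.
; That event spawns a BP_Wall at the given location and rotation.
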(event `self.ReceiveBeginPlay`)

(event `self.ReceiveActorBeginOverlap`
  (params (OtherActor :type "Actor Object Reference")))

(event `self.ReceiveTick`
  (params (DeltaSeconds :type "Float (single-precision)"))
  (`parent.ReceiveTick` 0.0))

(event `self.OverrideThis`
  (`self.spawnWall` (+ (* (`self.GetActorForwardVector`) 1000.0) (`self.K2_GetActorLocation`)) (`self.K2_GetActorRotation`)))

(event `spawnWall`
  (params (`Spawn Transform Location` :type "Vector Structure") (`Spawn Transform Rotation` :type "Rotator Structure"))
  (`|SpawnActorFromClass` "/Game/Ship/Abilities/TestWall/BP_Wall.BP_Wall_C" (`KismetMathLibrary.MakeTransform` `Spawn Transform Location` `Spawn Transform Rotation`) "Undefined" "OverrideRootScale"))

(fn `UserConstructionScript`
  (`parent.UserConstructionScript`))