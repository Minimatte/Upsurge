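; Base ship ability actor that provides shared cooldown handling for child abilities.
; Tick counts the current cooldown down to zero, and UseAbility restarts it at the maximum before calling OverrideThis.
; OverrideThis is the hook for child behavior and only prints a placeholder message here.
; On BeginPlay it binds to the owning BP_Ship's destroyed event so it destroys itself with the ship.
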(event `self.ReceiveBeginPlay`
  (add `self.OnDestroyed` (cast `/Game/BP_Ship` (`self.GetOwner`) :!pure true) (delegate `DestroyThis`)))

(event `DestroyThis`
  (`self.K2_DestroyActor`))

(event `self.ReceiveTick`
  (params (DeltaSeconds :type "Float (single-precision)"))
  (if (> (`self.CurrentCooldown`) 0.0)
    (set `self.CurrentCooldown` (`KismetMathLibrary.FClamp` (- (`self.CurrentCooldown`) DeltaSeconds) 0.0 (`self.MaxCooldown`)))))

(event `UseAbility`
  (if (<= (`self.CurrentCooldown`) 0.0)
    (set `self.CurrentCooldown` (`self.MaxCooldown`))
    (`self.OverrideThis`)))

(event `OverrideThis`
  (`KismetSystemLibrary.PrintString` "There is nothing in this Ability"))

(fn `UserConstructionScript`)