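; Test ship ability that deploys a Turret actor at the ability actor's location.
; The OverrideThis event passes the ability's owner to spawnTurret, which spawns only with network authority and ignores collisions.
; The owner, cast to Pawn, becomes the turret's Owner and Instigator.
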(event `self.ReceiveBeginPlay`)

(event `self.ReceiveActorBeginOverlap`
  (params (OtherActor :type "Actor Object Reference")))

(event `self.ReceiveTick`
  (params (DeltaSeconds :type "Float (single-precision)"))
  (`parent.ReceiveTick` 0.0))

(event `self.OverrideThis`
  (`self.spawnTurret` (`self.GetOwner`)))

(event `spawnTurret`
  (params (Object :type "Object Object Reference"))
  (bind _aspawn (cast `Pawn` Object :!pure true))
  (`/Engine/EditorBlueprintResources/ActorMacros.Switch Has Authority`
    (:`Authority`
      (`|SpawnActorFromClass` "/Game/Ship/Turret/Turret.Turret_C" (`KismetMathLibrary.MakeTransform` (`self.K2_GetActorLocation`)) "AlwaysSpawn" "OverrideRootScale" _aspawn _aspawn))))

(fn `UserConstructionScript`
  (`parent.UserConstructionScript`))