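; BP_Ability_Mines is a ship ability that drops a mine behind the ship.
; It overrides the parent's OverrideThis event to compute a spawn point a fixed distance opposite the actor's forward vector.
; That event passes the location, damage, instigator and the instigator controller's pawn as owner to a spawnMine event, which spawns the BP_Mine actor.
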(event `spawnMine`
  (params (`Spawn Transform Location` :type "Vector Structure") (Owner :type "Actor Object Reference") (Damage :type "Float (double-precision)") (Instigator :type "Pawn Object Reference"))
  (`|SpawnActorFromClass` "/Game/Ship/Abilities/Blueprints/BP_Mine.BP_Mine_C" (`KismetMathLibrary.MakeTransform` `Spawn Transform Location`) "Undefined" "OverrideRootScale" Owner Damage Instigator))

(event `self.OverrideThis`
  (`self.spawnMine` (+ (`self.K2_GetActorLocation`) (* (`self.GetActorForwardVector`) -1300.0)) (`Controller.K2_GetPawn` (`self.GetInstigatorController`)) (`self.Damage`) (`self.GetInstigator`)))

(fn `UserConstructionScript`
  (`parent.UserConstructionScript`))