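; Ship ability mine that spins randomly and explodes when a ship other than its instigator touches it.
; Any damage also detonates it after a short delay, so nearby mines can chain-react.
; Detonation runs on authority: it spawns the explosion effect, waits briefly, then deals full radial damage credited to the instigator.
; The mine destroys itself only if that damage call reports a hit.
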(event `self.ReceiveBeginPlay`
  (`/Engine/EditorBlueprintResources/ActorMacros.Switch Has Authority`
    (:`Authority`
      (set `RotatingMovementComponent.RotationRate` (`KismetMathLibrary.MakeRotator` (`KismetMathLibrary.RandomFloatInRange` 45.0 -45.0) (`KismetMathLibrary.RandomFloatInRange` 45.0 -45.0) (`KismetMathLibrary.RandomFloatInRange` 45.0 -45.0)) (`self.RotatingMovement`)))))

(event `self.Collision.OnComponentBeginOverlap`
  (params (OtherActor :type "Actor Object Reference") (OtherComp :type "PrimitiveComponent Object Reference") (OtherBodyIndex :type Integer) (bFromSweep :type Boolean) (SweepResult :type "HitResult Structure (by ref)"))
  (if (and (== (`GameplayStatics.GetObjectClass` OtherActor) "/Game/BP_Ship.BP_Ship_C") (!= OtherActor (`self.GetInstigator`)))
    (`/Engine/EditorBlueprintResources/ActorMacros.Switch Has Authority` :!label _label
      (:`Authority`
        (`self.MakeEffect` "/Game/Ship/Abilities/Mine/Particle/P_Ability_Mine_Explosion.P_Ability_Mine_Explosion" (`self.K2_GetActorLocation`))
        (`KismetSystemLibrary.Delay` 0.2)
        (bind _returnvalue (`GameplayStatics.ApplyRadialDamage` (`self.Damage`) (`self.K2_GetActorLocation`) 1024.0 "/Script/Engine.DamageType" (`|MakeArray` self :!type "Actor Object Reference") (`self.GetInstigator`) (`self.GetInstigatorController`) true))
        (if _returnvalue
          (`self.K2_DestroyActor`))))))

(event `self.ReceiveAnyDamage`
  (params (Damage :type "Float (single-precision)") (DamageType :type "DamageType Object Reference") (InstigatedBy :type "Controller Object Reference") (DamageCauser :type "Actor Object Reference"))
  (`KismetSystemLibrary.Delay` 0.1)
  (goto _label))

(event `MakeEffect`
  (params (EmitterTemplate :type "ParticleSystem Object Reference") (Location :type "Vector Structure"))
  (`GameplayStatics.SpawnEmitterAtLocation` EmitterTemplate Location))

(fn `UserConstructionScript`)