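; BP_Ability_TESTEMP is a test ship ability that fires an EMP burst from its owner's location.
; OverrideThis calls Emp, which on authority runs a fixed-radius multi-sphere object trace that ignores the owner and leaves persistent debug drawing.
; It spawns an explosion emitter at the origin and zeroes defensive and offensive charge in each hit BP_Ship's PlayerState charge system.
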(event `self.ReceiveBeginPlay`)

(event `self.OverrideThis`
  (`self.emp` (`self.K2_GetActorLocation` (`self.GetOwner`)) (`self.GetOwner`)))

(event `self.ReceiveActorBeginOverlap`
  (params (OtherActor :type "Actor Object Reference")))

(event `self.ReceiveTick`
  (params (DeltaSeconds :type "Float (single-precision)"))
  (`parent.ReceiveTick` 0.0))

(event `emp`
  (params (Start :type "Vector Structure") (`[0]` :type "Actor Object Reference"))
  (`/Engine/EditorBlueprintResources/ActorMacros.Switch Has Authority`
    (:`Authority`
      (bind _outhits (`KismetSystemLibrary.SphereTraceMultiForObjects` Start (+ Start (0.0 0.0 1.0)) 1024.0 (`|MakeArray` "ObjectTypeQuery7" :!type "EObjectTypeQuery Enum") false (`|MakeArray` `[0]`) "Persistent"))
      (`self.SpawnEffect` Start)
      (for _array_element _outhits
        (`self.setCharges` (`.HitActor` (`GameplayStatics.BreakHitResult` _array_element)))))))

(event `setCharges`
  (params (Object :type "Object Object Reference"))
  (bind _asbp_ship (cast `/Game/BP_Ship` Object))
  (bind _bp_chargesystem (`/Game/Networking/ShipPlayerState.BP_ChargeSystem` (cast `/Game/Networking/ShipPlayerState` (`Pawn.PlayerState` _asbp_ship) :!pure true)))
  (set `/Game/Ship/BP_ChargeSystem.DefensiveCharge` 0.0 _bp_chargesystem)
  (set `/Game/Ship/BP_ChargeSystem.OffensiveCharge` 0.0 _bp_chargesystem))

(event `SpawnEffect`
  (params (Location :type "Vector Structure"))
  (`GameplayStatics.SpawnEmitterAtLocation` "/Game/Ship/Abilities/EMP/P_EMP_Exploson.P_EMP_Exploson" Location))

(fn `UserConstructionScript`
  (`parent.UserConstructionScript`))