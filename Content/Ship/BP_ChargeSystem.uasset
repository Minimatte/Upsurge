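; Ship charge system that manages offensive, defensive and shield energy pools, all capped by the ship's power core charge.
; Tick refills each pool in proportion to core charge, shield slowest, while spending from a pool pauses its regen through a cooldown timer.
; Core charge sets the level per hundred points; crossing a threshold upward calls LevelUp on the ship, and either direction triggers the player controller's weapon spawn event.
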(event Custom|SpentDefensiveCharge
  (Variables|Defensive|SetDefensiveChargeBlocker true)
  (Utilities|Time|SetTimerbyFunctionName 0 "UnBlockDefensiveCharge" (Variables|Defensive|GetDefensiveCooldown)))

(event Custom|SpentOffensiveCharge
  (Variables|Offensive|SetOffensiveChargeBlocker true)
  (Utilities|Time|SetTimerbyFunctionName 0 "UnblockOffensiveCharge" (Variables|Offensive|GetOffensiveCooldown)))

(event Custom|UnBlockDefensiveCharge
  (Variables|Defensive|SetDefensiveChargeBlocker false))

(event Custom|UnblockOffensiveCharge
  (Variables|Offensive|SetOffensiveChargeBlocker false))

(event Custom|CallForServerWeWinMaybe
  (params (CurrentLevel :type Float%20%28single-precision%29) (PlayerShip :type Actor%20Object%20Reference))
  (Default|CheckforWinner (.AsGM%20Main%20Game%20Mode (Utilities|Casting|CastToGM_MainGameMode (Game|GetGameMode)))))

(event Custom|SpentShieldCharge
  (Variables|Shield|SetShieldChargeBlocker true)
  (Utilities|Time|SetTimerbyFunctionName 0 "UnblockShieldCharge" (Variables|Shield|GetShieldCooldown)))

(event Custom|UnblockShieldCharge
  (Variables|Shield|SetShieldChargeBlocker false))

(event EventTick
  (params (DeltaSeconds :type Float%20%28single-precision%29))
  (Utilities|FlowControl|Sequence
    (:then_0
      (if (not (Variables|Defensive|GetDefensiveChargeBlocker))
        (CallFunction|UpdateDefensiveCharge (/ (* (Utilities|Time|GetWorldDeltaSeconds) (Variables|General|GetPowerCoreCharge)) 2.0))))
    (:then_1
      (if (not (Variables|Offensive|GetOffensiveChargeBlocker))
        (CallFunction|UpdateOffensiveCharge (/ (* (Utilities|Time|GetWorldDeltaSeconds) (Variables|General|GetPowerCoreCharge)) 2.0))))
    (:then_2
      (if (not (Variables|Shield|GetShieldChargeBlocker))
        (CallFunction|UpdateShieldCharge (/ (* (Utilities|Time|GetWorldDeltaSeconds) (Variables|General|GetPowerCoreCharge)) 6.0))))))

(event EventBeginPlay
  (CallFunction|InitializeCurrentCharges))

(fn InitializeCurrentCharges
  (Utilities|FlowControl|Sequence
    (:then_0
      (Variables|Offensive|SetOffensiveCharge (Variables|General|GetPowerCoreCharge)))
    (:then_1
      (Variables|Defensive|SetDefensiveCharge (Variables|General|GetPowerCoreCharge)))
    (:then_2
      (Variables|Shield|SetShieldCharge (Variables|General|GetPowerCoreCharge)))))

(fn UpdatePowerCoreCharge
  (params (Amount%20%28+/-%29 :type Float%20%28single-precision%29) (ship :type Ship%20Player%20Controller%20Object%20Reference))
  (LocalVariables|SetOriginalCharge (Variables|General|GetPowerCoreCharge))
  (bind _output_get (Variables|General|SetPowerCoreCharge (Math|Float|Clamp(Float) (+ (Variables|General|GetPowerCoreCharge) Amount%20%28+/-%29) 1e+02 (Variables|General|GetPowerCoreMaximum))))
  (Math|Float|CompareFloat _output_get (LocalVariables|GetOriginalCharge)
    (:>
      _)
    (:==
      _)
    (:<
      _))
  (Math|Integer|CompareInt (Math|Float|Floor (/ (Variables|General|GetPowerCoreCharge) 1e+02)) (Math|Float|Floor (/ (LocalVariables|GetOriginalCharge) 1e+02))
    (:>
      (Default|LevelUp ship (.AsBP%20Ship (Utilities|Casting|CastToBP_Ship (Pawn|GetControlledPawn ship))))
      (if (Networking|IsServer)
        _
        (else
          _))
      (Default|NewSpawnWeaponEvent (.AsShip%20Player%20Controller (Utilities|Casting|CastToShipPlayerController (Pawn|GetController (Game|GetPlayerCharacter 0)))) :!label _label))
    (:==
      _)
    (:<
      (goto _label)))
  (Utilities|FlowControl|Sequence
    (:then_0
      (if (> (Variables|Offensive|GetOffensiveCharge) (Variables|General|GetPowerCoreCharge))
        (Variables|Offensive|SetOffensiveCharge (Variables|General|GetPowerCoreCharge))))
    (:then_1
      (if (> (Variables|Defensive|GetDefensiveCharge) (Variables|General|GetPowerCoreCharge))
        (Variables|Defensive|SetDefensiveCharge (Variables|General|GetPowerCoreCharge))))))

(fn UpdateDefensiveCharge
  (params (Amount%20%28+/-%29 :type Float%20%28single-precision%29))
  (Math|Float|CompareFloat Amount%20%28+/-%29 0.0
    (:>
      (if (< (Variables|Defensive|GetDefensiveCharge) (Variables|General|GetPowerCoreCharge))
        (Variables|Defensive|SetDefensiveCharge (Math|Float|Clamp(Float) (+ (Variables|Defensive|GetDefensiveCharge) Amount%20%28+/-%29) 0.0 (Variables|General|GetPowerCoreCharge)) :!label _label)))
    (:<
      (if (> (Variables|Defensive|GetDefensiveCharge) 0.0)
        (CallFunction|SpentDefensiveCharge)
        (goto _label)))))

(fn UpdateOffensiveCharge
  (params (Amount%20%28+/-%29 :type Float%20%28single-precision%29))
  (Math|Float|CompareFloat Amount%20%28+/-%29 0.0
    (:>
      (if (< (Variables|Offensive|GetOffensiveCharge) (Variables|General|GetPowerCoreCharge))
        (Variables|Offensive|SetOffensiveCharge (Math|Float|Clamp(Float) (+ (Variables|Offensive|GetOffensiveCharge) Amount%20%28+/-%29) 0.0 (Variables|General|GetPowerCoreCharge)) :!label _label)))
    (:<
      (if (> (Variables|Offensive|GetOffensiveCharge) 0.0)
        (CallFunction|SpentOffensiveCharge)
        (goto _label)))))

(fn GetCurrentLevel
  (return (Math|Float|Truncate (/ (Variables|General|GetPowerCoreCharge) 1e+02))))

(fn UpdateShieldCharge
  (params (Amount%20%28+/-%29 :type Float%20%28single-precision%29))
  (Math|Float|CompareFloat Amount%20%28+/-%29 0.0
    (:>
      (if (< (Variables|Shield|GetShieldCharge) (Variables|General|GetPowerCoreCharge))
        (Variables|Shield|SetShieldCharge (Math|Float|Clamp(Float) (+ (Variables|Shield|GetShieldCharge) Amount%20%28+/-%29) 0.0 (Variables|General|GetPowerCoreCharge)) :!label _label)))
    (:<
      (if (> (Variables|Shield|GetShieldCharge) 0.0)
        (CallFunction|SpentShieldCharge)
        (goto _label)))))