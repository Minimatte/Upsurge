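; Component that grants and triggers a ship's abilities, adding ability 0 at BeginPlay.
; AddAbility runs only with owner authority, spawning the class from Abilities as an actor attached to the owner and appending it to CurrentAbilites.
; UseAbility forwards to the BP_Ability_Base instance at that index, so indices match IDs only when abilities are added in ID order.
; GetAbility looks up the class by ID.
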(event `UseAbility`
  (params (AbilityID :type Integer))
  (bind _item (`KismetArrayLibrary.Array_Get` (`self.CurrentAbilites`) AbilityID))
  (`/Engine/EditorBlueprintResources/StandardMacros.IsValid` _item
    (:`Is Valid`
      (`/Game/Ship/Abilities/BP_Ability_Base.UseAbility` _item))))

(event `AddAbility`
  (params (AbilityID :type Integer))
  (bind _returnvalue (`self.GetOwner`))
  (`/Engine/EditorBlueprintResources/StandardMacros.IsValid` (`self.GetOwner`)
    (:`Is Valid`
      (if (`Actor.HasAuthority` (`self.GetOwner`))
        (`/Engine/EditorBlueprintResources/StandardMacros.IsValid` (`KismetArrayLibrary.Array_Get` (`self.CurrentAbilites`) AbilityID)
          (:`Is Not Valid`
            (bind _returnvalue_2 (`|SpawnActorFromClass` (`KismetArrayLibrary.Array_Get` (`self.Abilities`) AbilityID) (`KismetMathLibrary.MakeTransform` (`Actor.K2_GetActorLocation` _returnvalue)) "Undefined" "OverrideRootScale" _returnvalue (cast `Pawn` _returnvalue :!pure true)))
            (`Actor.K2_AttachRootComponentToActor` _returnvalue_2 (`self.GetOwner`) "None" "SnapToTargetIncludingScale" true)
            (`KismetArrayLibrary.Array_Add` (`self.CurrentAbilites`) (cast `/Game/Ship/Abilities/BP_Ability_Base` _returnvalue_2 :!pure true))))))))

(event `self.ReceiveBeginPlay`
  (`self.AddAbility` 0))

(fn `GetAbility`
  (params (AbilityID :type Integer))
  (returns (Item :type "Actor Class Reference"))
  (return (`KismetArrayLibrary.Array_Get` (`self.Abilities`) AbilityID)))