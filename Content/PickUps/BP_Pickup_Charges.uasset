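; Charge pickup that homes in on a ship and gives it power charges and score, ignoring the ship of its ControllerOwner.
; On the server, SuctionArea locks onto the first eligible BP_Ship as Target, and Tick moves the pickup toward it with a swept offset.
; Collision overlap adds charges to the touching ship, spawns particles and adds multiplied score on Target, then destroys the pickup.
; Full-charge checks are left disconnected.
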(event `self.Collision.OnComponentBeginOverlap`
  (params (OtherActor :type "Actor Object Reference") (OtherComp :type "PrimitiveComponent Object Reference") (OtherBodyIndex :type Integer) (bFromSweep :type Boolean) (SweepResult :type "HitResult Structure (by ref)"))
  (bind _asbp_ship (cast `/Game/BP_Ship` OtherActor :!pure true))
  (bind _returnvalue (`self.GetInstigatorController` _asbp_ship))
  (`/Engine/EditorBlueprintResources/ActorMacros.Switch Has Authority`
    (:`Authority`
      (if (and (== (`GameplayStatics.GetObjectClass` OtherActor) "/Game/BP_Ship.BP_Ship_C") (!= (`Controller.PlayerState` (`self.GetInstigatorController` OtherActor)) (`self.controllerOwner`)))
        (`/Game/BP_Ship.AddChargesServer` _asbp_ship (`KismetMathLibrary.Conv_IntToDouble` (`self.ExperienceToGivePlayer`)) (`Controller.PlayerState` _returnvalue) (cast `/Game/ShipPlayerController` _returnvalue :!pure true))
        (`self.spawn particle` (`self.Target`))
        (`self.AddScoreServer`)
        (`self.K2_DestroyActor`)))))

(event `AddScoreServer`
  (`/Game/Networking/ShipPlayerState.AddScore` (cast `/Game/Networking/ShipPlayerState` (`Pawn.PlayerState` (`self.Target`)) :!pure true) (* (`self.ExperienceToGivePlayer`) 3.0)))

(event `self.SuctionArea.OnComponentBeginOverlap`
  (params (OtherActor :type "Actor Object Reference") (OtherComp :type "PrimitiveComponent Object Reference") (OtherBodyIndex :type Integer) (bFromSweep :type Boolean) (SweepResult :type "HitResult Structure (by ref)"))
  (`/Engine/EditorBlueprintResources/ActorMacros.Switch Has Authority`
    (:`Authority`
      (if (and (== (`GameplayStatics.GetObjectClass` OtherActor) "/Game/BP_Ship.BP_Ship_C") (!= (`Controller.PlayerState` (`self.GetInstigatorController` OtherActor)) (`self.controllerOwner`)))
        (`/Engine/EditorBlueprintResources/StandardMacros.IsValid` (`self.Target`)
          (:`Is Not Valid`
            (set `self.Target` (cast `/Game/BP_Ship` OtherActor :!pure true))))))))

(event `spawn particle`
  (params (ship :type "/Game/BP_Ship Object Reference"))
  (`/Game/BP_Ship.spawn particle Pickup core` ship (`/Game/BP_Ship.ShipMesh` ship) (`self.K2_GetActorLocation` ship)))

(event `self.ReceiveTick`
  (params (DeltaSeconds :type "Float (single-precision)"))
  (`/Engine/EditorBlueprintResources/ActorMacros.Switch Has Authority`
    (:`Authority`
      (`/Engine/EditorBlueprintResources/StandardMacros.IsValid` (`self.Target`)
        (:`Is Valid`
          (`self.K2_AddActorWorldOffset` (* (`KismetMathLibrary.Normal` (- (`self.K2_GetActorLocation` (`self.Target`)) (`self.K2_GetActorLocation`))) 50.0) true))))))

(fn `UserConstructionScript`)