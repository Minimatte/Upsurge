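; Overcharge pickup that temporarily sets the collecting ship's player to max level through its charge system.
; On overlap, the authority accepts only a BP_Ship whose instigator PlayerState differs from ControllerOwner, then applies the boost once, adds score and destroys the pickup.
; On BeginPlay it creates a pickup pointer widget and adds it to the viewport.
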(event `self.ReceiveTick`
  (params (DeltaSeconds :type "Float (single-precision)"))
  (`parent.ReceiveTick` 0.0))

(event `self.Collision.OnComponentBeginOverlap`
  (params (OtherActor :type "Actor Object Reference") (OtherComp :type "PrimitiveComponent Object Reference") (OtherBodyIndex :type Integer) (bFromSweep :type Boolean) (SweepResult :type "HitResult Structure (by ref)"))
  (bind _asship_player_state (cast `/Game/Networking/ShipPlayerState` (`Pawn.PlayerState` (cast `/Game/BP_Ship` OtherActor :!pure true)) :!pure true))
  (if (== (`GameplayStatics.GetObjectClass` OtherActor) "/Game/BP_Ship.BP_Ship_C")
    (`/Engine/EditorBlueprintResources/ActorMacros.Switch Has Authority`
      (:`Authority`
        (if (and (== (`GameplayStatics.GetObjectClass` OtherActor) "/Game/BP_Ship.BP_Ship_C") (!= (`Controller.PlayerState` (`self.GetInstigatorController` OtherActor)) (`self.controllerOwner`)))
          (`/Engine/EditorBlueprintResources/StandardMacros.DoOnce` false
            (:`Completed`
              (`/Game/Networking/ShipPlayerState.SetPlayerToMaxLevelTemporary` _asship_player_state (`/Game/Networking/ShipPlayerState.BP_ChargeSystem` _asship_player_state))
              (`self.AddScoreServer`)
              (`self.K2_DestroyActor`))))))))

(event `SpawnWidgetForEveryone`
  (bind _returnvalue (`|CreateWidget` "/Game/GUI/W_PickupPointer.W_PickupPointer_C" null self))
  (`UserWidget.AddToViewport` _returnvalue 0))

(event `self.ReceiveBeginPlay`
  (`self.SpawnWidgetForEveryone`))

(fn `UserConstructionScript`
  (`parent.UserConstructionScript`))