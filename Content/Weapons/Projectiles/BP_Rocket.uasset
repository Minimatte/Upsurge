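; BP_Rocket is a rocket projectile with optional homing and area damage.
; When homing is enabled, Tick ramps up the projectile movement's homing acceleration.
; On destruction it spawns an impact effect, and the server applies full radial damage once, ignoring the owner.
; An OnRep handler interpolates toward a replicated location with a swept move, but the server code setting that location is unconnected.
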(event `self.ReceiveTick`
  (params (DeltaSeconds :type "Float (single-precision)"))
  (bind _projectilemovement (`self.ProjectileMovement`))
  (if (`self.IsHomingProjectile`)
    (set `ProjectileMovementComponent.HomingAccelerationMagnitude` (`KismetMathLibrary.FInterpTo` (`ProjectileMovementComponent.HomingAccelerationMagnitude` _projectilemovement) 25000.0 DeltaSeconds 8.0) _projectilemovement)))

(event `self.ReceiveDestroyed`
  (bind _returnvalue (`self.GetOwner`))
  (bind _returnvalue_2 (`self.K2_GetActorLocation`))
  (`self.MakeEffect` (`self.impactParticle`) _returnvalue_2)
  (`/Engine/EditorBlueprintResources/ActorMacros.Switch Has Authority`
    (:`Authority`
      (`/Engine/EditorBlueprintResources/StandardMacros.DoOnce` false
        (:`Completed`
          (`GameplayStatics.ApplyRadialDamage` (`self.damage`) _returnvalue_2 1300.0 null (`|MakeArray` _returnvalue) _returnvalue (`self.GetInstigatorController`) true))))))

(fn `OnRep_actualLocation`
  (`self.K2_SetActorLocation` (`KismetMathLibrary.VInterpTo` (`self.K2_GetActorLocation`) (`self.actualLocation`) (`GameplayStatics.GetWorldDeltaSeconds`) 10000.0) true)
  (if (`self.HasAuthority`)
    _))

(fn `UserConstructionScript`
  (`parent.UserConstructionScript`))