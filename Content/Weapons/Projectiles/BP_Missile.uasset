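; Homing missile projectile that seeks ships and explodes with radial damage when destroyed.
; The first non-instigator BP_Ship entering its box becomes the ProjectileMovement homing target.
; Each tick, homing acceleration ratchets up as distance to the target shrinks from the lock-on distance, never easing off.
; Destruction spawns the impact effect and applies server-only damage sparing the owner; an OnRep interpolates toward ActualLocation, but the graph setting that variable is disconnected.
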(event `self.Box.OnComponentBeginOverlap`
  (params (OtherActor :type "Actor Object Reference") (OtherComp :type "PrimitiveComponent Object Reference") (OtherBodyIndex :type Integer) (bFromSweep :type Boolean) (SweepResult :type "HitResult Structure (by ref)"))
  (bind _asbp_ship (cast `/Game/BP_Ship` OtherActor :!pure true))
  (if (and (== (`GameplayStatics.GetObjectClass` OtherActor) "/Game/BP_Ship.BP_Ship_C") (!= OtherActor (`self.Instigator`)))
    (`/Engine/EditorBlueprintResources/StandardMacros.DoOnce` false
      (:`Completed`
        (set `self.HomingTarget` _asbp_ship)
        (set `ProjectileMovementComponent.HomingTargetComponent` (`Character.Mesh` _asbp_ship) (`self.ProjectileMovement`))
        (set `self.StartingDistance` (`self.GetDistanceTo` (`self.HomingTarget`) self))))))

(event `self.ReceiveTick`
  (params (DeltaSeconds :type "Float (single-precision)"))
  (bind _returnvalue (`KismetMathLibrary.Lerp` 300000.0 1000.0 (/ (`self.GetDistanceTo` (`self.HomingTarget`) self) (`self.StartingDistance`))))
  (`self.HomingTarget`
    (:`then`
      (if (> _returnvalue (`ProjectileMovementComponent.HomingAccelerationMagnitude` (`self.ProjectileMovement`)))
        (set `ProjectileMovementComponent.HomingAccelerationMagnitude` _returnvalue (`self.ProjectileMovement`))))
    (:`else`)))

(event `self.ReceiveDestroyed`
  (bind _returnvalue (`self.GetOwner`))
  (bind _returnvalue_2 (`self.K2_GetActorLocation`))
  (`self.MakeEffect` (`self.impactParticle`) _returnvalue_2)
  (`/Engine/EditorBlueprintResources/ActorMacros.Switch Has Authority`
    (:`Authority`
      (`/Engine/EditorBlueprintResources/StandardMacros.DoOnce` false
        (:`Completed`
          (`GameplayStatics.ApplyRadialDamage` (`self.damage`) _returnvalue_2 300.0 null (`|MakeArray` _returnvalue) _returnvalue (`self.GetInstigatorController`) true))))))

(fn `OnRep_actualLocation`
  (`self.K2_SetActorLocation` (`KismetMathLibrary.VInterpTo` (`self.K2_GetActorLocation`) (`self.actualLocation`) (`GameplayStatics.GetWorldDeltaSeconds`) 10000.0) true)
  (if (`self.HasAuthority`)
    _))

(fn `UserConstructionScript`
  (`parent.UserConstructionScript`))