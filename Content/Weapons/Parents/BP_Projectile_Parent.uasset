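; Parent projectile Blueprint for weapons, with a set lifespan, velocity, spawn sound and optional homing on a locked BP_Ship's mesh.
; On overlapping anything but its instigator, the server applies damage once with authority, plays the destroy sound and destroys the projectile, while non-servers just destroy it.
; The Destroyed event spawns the impact particle, so the effect also appears when the lifespan expires.
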(event `self.ReceiveBeginPlay`
  (bind _projectilemovement (`self.ProjectileMovement`))
  ;[1 1 1] Life
  (`self.SetLifeSpan` (`self.duration`))
  ;[1 1 1] Update velocity
  (set `MovementComponent.Velocity` (`self.SpeedVectorTest`) (`self.ProjectileMovement`))
  ;[1 1 1] Spawn Sound
  (`self.PlaySoundSpawnEffect` (`self.SoundEffectSpawn`) (`self.K2_GetActorLocation`))
  (if (`self.IsHomingProjectile`)
    (set `ProjectileMovementComponent.bIsHomingProjectile` true _projectilemovement)
    ;[1 1 1] If the player has a target - set it as the homing target
    (bind _lockedtarget (`self.LockedTarget`)
      (:`then`
        (set `ProjectileMovementComponent.HomingTargetComponent` (`Character.Mesh` (cast `/Game/BP_Ship` _lockedtarget :!pure true)) _projectilemovement))
      (:`else`))))

(event `self.Collision.OnComponentBeginOverlap`
  (params (OtherActor :type "Actor Object Reference") (OtherComp :type "PrimitiveComponent Object Reference") (OtherBodyIndex :type Integer) (bFromSweep :type Boolean) (SweepResult :type "HitResult Structure (by ref)"))
  (if (!= OtherActor (`self.GetInstigator`))
    (if (`KismetSystemLibrary.IsServer`)
      (`/Engine/EditorBlueprintResources/ActorMacros.Switch Has Authority`
        (:`Authority`
          (`/Engine/EditorBlueprintResources/StandardMacros.DoOnce` false
            (:`Completed`
              (`self.ApplyDamage` OtherActor)
              ;[1 1 1] Sound: Only runs if it hits a wall - ofc
              (`self.PlaySoundDeathEffect` (`self.SoundEffectDestroy`) (`self.K2_GetActorLocation`))))))
      (else
        (`self.K2_DestroyActor`)))))

(event `ApplyDamage`
  (params (DamagedActor :type "Actor Object Reference"))
  (`/Engine/EditorBlueprintResources/ActorMacros.Switch Has Authority`
    (:`Authority`
      (`GameplayStatics.ApplyDamage` DamagedActor (`self.damage`) (`self.GetInstigatorController`) (`self.GetInstigator`))
      (`self.K2_DestroyActor`))))

(event `MakeEffect`
  (params (EmitterTemplate :type "ParticleSystem Object Reference") (Location :type "Vector Structure"))
  (`GameplayStatics.SpawnEmitterAtLocation` EmitterTemplate Location))

(event `PlaySoundSpawnEffect`
  (params (Sound :type "SoundBase Object Reference") (Location :type "Vector Structure"))
  (`GameplayStatics.PlaySoundAtLocation` Sound Location))

(event `PlaySoundDeathEffect`
  (params (Sound :type "SoundBase Object Reference") (Location :type "Vector Structure"))
  (`GameplayStatics.PlaySoundAtLocation` Sound Location))

(event `self.ReceiveDestroyed`
  (`self.MakeEffect` (`self.impactParticle`) (`self.K2_GetActorLocation`)))

(fn `UserConstructionScript`)