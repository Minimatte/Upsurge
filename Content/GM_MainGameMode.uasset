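; Game mode for a timed multiplayer ship match won on score, tracking players and assigning IDs and colors at login.
; Respawns possess a new ship at a random PlayerStart, while kills destroy the pawn and drop a charge pickup scaled to the victim's power core.
; Tick feeds time left and score leader to the GameState, then once time expires announces the winner, destroys ships and calls ServerTravel.
; Server messages and kill logs fan out through each PlayerState.
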(event Custom|CheckForWinner
  (bind _playerstateinlead (CallFunction|CheckforPlayerinLeadScore))
  (bind _outactors (Actor|GetAllActorsOfClass "/Game/BP_Ship.BP_Ship_C"))
  (for _array_element _outactors
    (Default|ShowScoreScreenGameEnd (.AsShip%20Player%20Controller (Utilities|Casting|CastToShipPlayerController (Pawn|GetController _array_element))))
    (Variables|/Game/Networking/ShipPlayerState.ShipPlayerState_C|SetGameOver (.AsShip%20Player%20State (Utilities|Casting|CastToShipPlayerState (Variables|/Script/Engine.Controller|GetPlayerState (.AsShip%20Player%20Controller (Utilities|Casting|CastToShipPlayerController (Pawn|GetController _array_element)))))) true)
    (Actor|DestroyActor _array_element))
  (CallFunction|CreateServerMessage (Utilities|String|Append (Variables|/Game/Networking/ShipPlayerState.ShipPlayerState_C|GetMyPlayerName _playerstateinlead) " WINS!") false 1e+04)
  (Development|ExecuteConsoleCommand "ServerTravel Level_FinalLayoutDetailingV3?listen"))

(event Custom|CreateLogMessage
  (params (DisplayMessage :type String))
  (for _array_element (Variables|/Script/Engine.GameState|GetPlayerArray (Game|GetGameState))
    (Default|AddtoKillLog (.AsShip%20Player%20State (Utilities|Casting|CastToShipPlayerState _array_element)) DisplayMessage)))

(event Custom|CreateServerMessage
  (params (ServerMessage :type String) (Fadeout :type Boolean) (Fadetime :type Float%20%28single-precision%29))
  (for _array_element (Variables|/Script/Engine.GameState|GetPlayerArray (Game|GetGameState))
    (Default|CreateServerMessage (.AsShip%20Player%20State (Utilities|Casting|CastToShipPlayerState _array_element)) "/Game/GUI/W_ServerMessage.W_ServerMessage_C" ServerMessage Fadeout Fadetime)))

(event Custom|KillPlayer
  (params (PlayerController :type Ship%20Player%20Controller%20Object%20Reference))
  (bind _returnvalue (Pawn|GetControlledPawn PlayerController))
  (bind _playerstate (Variables|/Script/Engine.Controller|GetPlayerState PlayerController))
  (bind _asship_player_state (Utilities|Casting|CastToShipPlayerState _playerstate))
  (bind _bp_chargesystem (Variables|/Game/Networking/ShipPlayerState.ShipPlayerState_C|GetBP_ChargeSystem _asship_player_state))
  (bind _powercorecharge (Variables|/Game/Ship/BP_ChargeSystem.BP_ChargeSystem_C|GetPowerCoreCharge _bp_chargesystem))
  (bind _returnvalue_2 (* _powercorecharge 0.2))
  (Variables|Default|SetTempPlayerLocation (Transformation|GetActorLocation _returnvalue))
  (Actor|DestroyActor _returnvalue)
  (Game|SpawnActorfromClass "/Game/PickUps/BP_Pickup_Charges.BP_Pickup_Charges_C" (Math|Transform|MakeTransform (Variables|Default|GetTempPlayerLocation) "0, 0, 0" "1,1,1") "Undefined" 0 (Math|Integer|SelectInt (Math|Float|Truncate _returnvalue_2) 25 (> _returnvalue_2 25.0)) (Variables|/Script/Engine.Controller|GetPlayerState PlayerController)))

(event Custom|RespawnPlayer
  (params (playerController :type Ship%20Player%20Controller%20Object%20Reference))
  (bind _outactors (Actor|GetAllActorsOfClass "/Script/Engine.PlayerStart"))
  (Utilities|Array|Shuffle _outactors)
  (bind _returnvalue (Game|SpawnActorfromClass "/Game/BP_Ship.BP_Ship_C" (Math|Transform|MakeTransform (Transformation|GetActorLocation (Utilities|Array|Get(acopy) _outactors)) (Transformation|GetActorRotation (Utilities|Array|Get(acopy) _outactors)) "1,1,1") "AlwaysSpawn" playerController 0))
  (Pawn|Possess playerController _returnvalue)
  (Variables|/Game/ShipPlayerController.ShipPlayerController_C|SetPlayerRef playerController _returnvalue)
  (Utilities|Array|Clear (Variables|/Game/ShipPlayerController.ShipPlayerController_C|GetPrimaryWeaponsRef playerController))
  (Utilities|Array|Clear (Variables|/Game/ShipPlayerController.ShipPlayerController_C|GetSecondaryWeaponsRef playerController))
  (Default|InitializeCurrentCharges (Variables|/Game/Networking/ShipPlayerState.ShipPlayerState_C|GetBP_ChargeSystem (.AsShip%20Player%20State (Utilities|Casting|CastToShipPlayerState (Variables|/Script/Engine.Controller|GetPlayerState playerController))))))

(event Custom|SetPlayerToSpectate
  (params (PlayerController :type Ship%20Player%20Controller%20Object%20Reference))
  (Game|SpawnActorfromClass "/Game/PlayerRespawnPawn.PlayerRespawnPawn_C" (Math|Transform|MakeTransform "0, 0, 0" "0, 0, 0" "1,1,1") "Undefined" 0 0))

(event EventOnLogout
  (params (ExitingController :type Controller%20Object%20Reference))
  (Utilities|Array|RemoveItem (Variables|Default|GetCurrentPlayers) ExitingController))

(event EventPostLogin
  (params (NewPlayer :type Player%20Controller%20Object%20Reference))
  (bind _playerstate (Variables|/Script/Engine.Controller|GetPlayerState NewPlayer))
  (bind _asship_player_state (Utilities|Casting|CastToShipPlayerState _playerstate))
  (Utilities|Array|Add (Variables|Default|GetCurrentPlayers) NewPlayer)
  (bind _output_get (Variables|/Game/Networking/ShipPlayerState.ShipPlayerState_C|SetThisPlayerID _asship_player_state (- (Variables|Default|GetNumPlayers) 1)))
  (Default|SetPlayerColor _asship_player_state _output_get))

(event EventTick
  (params (DeltaSeconds :type Float%20%28single-precision%29))
  (bind _returnvalue (Utilities|Time|GetGameTimeinSeconds))
  (bind _secondstilgameisover (Variables|Default|GetSecondsTilGameIsOver))
  (bind _returnvalue_2 (Math|Conversions|ToFloat(Integer) _secondstilgameisover))
  (bind _returnvalue_3 (- _returnvalue_2 _returnvalue))
  (if (> _returnvalue_3 0.0)
    (Default|SetTimeLeft (.AsShip%20Game%20State (Utilities|Casting|CastToShipGameState (Game|GetGameState))) _returnvalue_3)
    (bind _playerstateinlead (CallFunction|CheckforPlayerinLeadScore))
    (Default|SetLeadingPlayer (.AsShip%20Game%20State (Utilities|Casting|CastToShipGameState (Game|GetGameState))) _playerstateinlead)
    (else
      (bind _playerstateinlead_2 (CallFunction|CheckforPlayerinLeadScore))
      (Default|SetLeadingPlayer (.AsShip%20Game%20State (Utilities|Casting|CastToShipGameState (Game|GetGameState))) _playerstateinlead_2)
      (Utilities|FlowControl|DoOnce false
        (:Completed
          (CallFunction|CheckforWinner))))))

(fn ConstructionScript)

(fn CheckforPlayerinLeadScore
  (for _array_element (Variables|Default|GetCurrentPlayers)
    (Utilities|IsValid (LocalVariables|GettempPlayerInLead)
      (:Is%20Valid
        (if (> (Variables|/Game/Networking/ShipPlayerState.ShipPlayerState_C|GetPlayerScore (.AsShip%20Player%20State (Utilities|Casting|CastToShipPlayerState (Variables|/Script/Engine.Controller|GetPlayerState _array_element)))) (Variables|/Game/Networking/ShipPlayerState.ShipPlayerState_C|GetPlayerScore (LocalVariables|GettempPlayerInLead)))
          (LocalVariables|SettempPlayerInLead (.AsShip%20Player%20State (Utilities|Casting|CastToShipPlayerState (Variables|/Script/Engine.Controller|GetPlayerState _array_element))))))
      (:Is%20Not%20Valid
        (LocalVariables|SettempPlayerInLead (.AsShip%20Player%20State (Utilities|Casting|CastToShipPlayerState (Variables|/Script/Engine.Controller|GetPlayerState _array_element)))))))
  (return (LocalVariables|GettempPlayerInLead)))

(fn CheckforPlayerinLeadPowerCores
  (bind _returnvalue (Game|GetGameState))
  (bind _playerarray (Variables|/Script/Engine.GameState|GetPlayerArray _returnvalue))
  (LocalVariables|SettempPlayerInLead (.AsShip%20Player%20State (Utilities|Casting|CastToShipPlayerState (Utilities|Array|Get(acopy) _playerarray))))
  (for _array_element _playerarray
    (if (> (.PowerCoreCharge (|CollapseGraph_0 _array_element)) (|CollapseGraph_1))
      (LocalVariables|SettempPlayerInLead (.AsShip%20Player%20State (|CollapseGraph_0 _array_element)))))
  (return (LocalVariables|GettempPlayerInLead)))